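; Test actor that exercises a custom event-listener system and config data table reads, logging what it receives.
; On BeginPlay it subscribes to a test event by both function name and delegate, and to an Inner-category TestUI event by delegate.
; The function-name handler logs every Item config row; the TestUI delegate converts its payload to a struct and prints the string.
; A function-name TestUI handler exists, but its registration is unwired.
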(event Custom|rec_bpEvent_test
  (bind _returnvalue (Class|WVBlueprintFunctionLibrary|GetConfig "Item"))
  (bind _outrownames (DataTable|GetDataTableRowNames _returnvalue))
  (for _array_element _outrownames
    (bind _returnvalue_2 (Utilities|GetDataTableRow _returnvalue _array_element)
      (:then
        (Class|WVBlueprintFunctionLibrary|LogI (Utilities|String|ToString(Text) (Utilities|Text|FormatText "{id}_{type}_{name}_{icon}" (.id (Utilities|Struct|BreakWVConfig_ItemRow _returnvalue_2)) (Utilities|Text|ToText(String) (.type (Utilities|Struct|BreakWVConfig_ItemRow _returnvalue_2))) (Utilities|Text|ToText(String) (.name (Utilities|Struct|BreakWVConfig_ItemRow _returnvalue_2))) (Utilities|Text|ToText(String) (Utilities|ToString(SoftObjectReference) (.icon (Utilities|Struct|BreakWVConfig_ItemRow _returnvalue_2)))))))))))

(event Custom|CustomEvent_0
  (params (obj :type WV%20Event%20Delegate%20Params%20One%20Structure%20%28by%20ref%29))
  (Class|WVBlueprintFunctionLibrary|LogI "rec BPEVENT_test"))

(event Custom|rec_InnerTestUI
  (params (data :type Test%20Multi%20Params%20Event%20Structure))
  (bind (_num_int32 _num_float _bval _str _obj) (Utilities|Struct|BreakTestMultiParamsEvent data))
  (Class|WVBlueprintFunctionLibrary|LogI (Utilities|String|ToString(Text) (Utilities|Text|FormatText "{num_int}_{num_float}_{bVal}_{str}_{obj}" _num_int32 _num_float (Math|Conversions|ToInteger(Boolean) _bval) (Utilities|Text|ToText(String) _str) (Utilities|Text|ToText(String) (Utilities|String|ToString(Object) _obj))))))

(event Custom|CustomEvent_3
  (params (obj :type WV%20Event%20Delegate%20Params%20One%20Structure%20%28by%20ref%29))
  (bind (_out _returnvalue) (Class|WVBlueprintFunctionLibrary|ConvEventOneParamstoStruct obj))
  (Class|WVBlueprintFunctionLibrary|LogI "rec InnerTestUI")
  (if _returnvalue
    (Development|PrintString (.str (Utilities|Struct|BreakTestMultiParamsEvent _out)))))

(event EventBeginPlay
  (Class|WVBlueprintFunctionLibrary|AddListenerFN "BPEVENT_test" "rec_bpEvent_test")
  (Class|WVBlueprintFunctionLibrary|AddListenerDL "BPEVENT_test" (delegate Custom|CustomEvent_0))
  (Class|WVBlueprintFunctionLibrary|AddListenerDLSP "Inner" "TestUI" (delegate Custom|CustomEvent_3)))

(event Collision|EventActorBeginOverlap
  (params (OtherActor :type Actor%20Object%20Reference)))

(event EventTick
  (params (DeltaSeconds :type Float%20%28single-precision%29)))

(fn ConstructionScript)