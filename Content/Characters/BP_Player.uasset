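; Player character Blueprint that handles camera look and movement from axis input.
; On BeginPlay it sets the control rotation to a slight downward pitch.
; Yaw and pitch input are scaled and applied only while the CompLockTarget component is not locking.
; Forward and right movement follow the control yaw, and apply only when the input magnitude falls within a configurable min/max range per axis.
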(event EventBeginPlay
  (bind _asplayer_controller (Utilities|Casting|CastToPlayerController (Pawn|GetController)))
  (Pawn|SetControlRotation _asplayer_controller (Math|Rotator|MakeRotator 0.0 -15.0 0.0)))

(event Collision|EventActorBeginOverlap
  (params (OtherActor :type Actor%20Object%20Reference)))

(event EventTick
  (params (DeltaSeconds :type Float%20%28single-precision%29)))

(event Input|AxisEvents|InputAxisRotationYaw
  (params (AxisValue :type Float%20%28single-precision%29))
  ;[1 1 1] Handle Input Rotation Yaw, Pitch
  (if (not (Class|LockTargetComp|IsLocking (Variables|Default|Get_Comp_LockTarget)))
    (Pawn|Input|AddControllerYawInput (* AxisValue (Variables|Default|GetAxisRotateYawScale)))))

(event Input|AxisEvents|InputAxisRotationPitch
  (params (AxisValue :type Float%20%28single-precision%29))
  ;[1 1 1] Handle Input Rotation Yaw, Pitch
  (if (not (Class|LockTargetComp|IsLocking (Variables|Default|Get_Comp_LockTarget)))
    (Pawn|Input|AddControllerPitchInput (* AxisValue (Variables|Default|GetAxisRotatePitchScale)))))

(event Input|AxisEvents|InputAxisMoveForward
  (params (AxisValue :type Float%20%28single-precision%29))
  (bind _returnvalue (Math|Float|Absolute(Float) AxisValue))
  (bind _axismoveforwardlimit (Variables|Default|GetAxisMoveForwardLimit))
  (bind (_x _y) (Math|Vector2D|BreakVector2D _axismoveforwardlimit))
  ;[1 1 1] Handle Input Move Forward, Right
  (if (and (>= _returnvalue _x) (<= _returnvalue _y))
    (Pawn|Input|AddMovementInput (Math|Vector|GetForwardVector (Math|Rotator|MakeRotator 0.0 0.0 (.Yaw (Math|Rotator|BreakRotator (Pawn|GetControlRotation :!class /Script/Engine.Pawn))))) AxisValue false)))

(event Input|AxisEvents|InputAxisMoveRight
  (params (AxisValue :type Float%20%28single-precision%29))
  (bind _returnvalue (Math|Float|Absolute(Float) AxisValue))
  (bind _axismoverightlimit (Variables|Default|GetAxisMoveRightLimit))
  (bind (_x _y) (Math|Vector2D|BreakVector2D _axismoverightlimit))
  ;[1 1 1] Handle Input Move Forward, Right
  (if (and (>= _returnvalue _x) (<= _returnvalue _y))
    (Pawn|Input|AddMovementInput (Math|Vector|GetRightVector (Math|Rotator|MakeRotator 0.0 0.0 (.Yaw (Math|Rotator|BreakRotator (Pawn|GetControlRotation :!class /Script/Engine.Pawn))))) AxisValue false)))

(fn ConstructionScript)