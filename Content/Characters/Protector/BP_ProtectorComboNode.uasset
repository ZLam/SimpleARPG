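; Combo node for the Protector character that plays the montage for the current combo step on its owning ActionCharacter.
; On Do, it finds the character's row in the Combo config DataTable, then looks up the combo name in its ComboInfoMap.
; The combo index selects play rate and optional section or start position, and the montage is loaded synchronously.
; A named section takes priority over start position; Condition defers to the parent.
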(event EventDo
  (|CallParentFunction)
  (bind _asaction_character (Utilities|Casting|CastToActionCharacter (Class|ComboNode|GetOwner)))
  (Variables|Default|SetActionCharacter _asaction_character)
  (bind _returnvalue (Class|WVBlueprintFunctionLibrary|GetConfig "Combo"))
  (bind _returnvalue_2 (Utilities|GetDataTableRow _returnvalue (Class|ActionCharacter|GetActionCharacterName (Variables|Default|GetActionCharacter)))
    (:then
      (if (.ReturnValue (Utilities|Map|Find (Utilities|Struct|BreakWVConfig_ComboRow _returnvalue_2) (Class|ComboNode|GetComboName)))
        (Variables|Default|SetRate (Utilities|Array|Get(acopy) (.Rates (Utilities|Struct|BreakWVConfig_ComboInfo (.Value (Utilities|Map|Find (Utilities|Struct|BreakWVConfig_ComboRow _returnvalue_2) (Class|ComboNode|GetComboName))))) (Class|ComboNode|GetComboIndex)))
        (if (> (Utilities|Array|Length (.Sections (Utilities|Struct|BreakWVConfig_ComboInfo (.Value (Utilities|Map|Find (Utilities|Struct|BreakWVConfig_ComboRow _returnvalue_2) (Class|ComboNode|GetComboName)))))) 0)
          (Variables|Default|SetSection (Utilities|Array|Get(acopy) (.Sections (Utilities|Struct|BreakWVConfig_ComboInfo (.Value (Utilities|Map|Find (Utilities|Struct|BreakWVConfig_ComboRow _returnvalue_2) (Class|ComboNode|GetComboName))))) (Class|ComboNode|GetComboIndex)))
          (if (> (Utilities|Array|Length (.StartPositions (Utilities|Struct|BreakWVConfig_ComboInfo (.Value (Utilities|Map|Find (Utilities|Struct|BreakWVConfig_ComboRow _returnvalue_2) (Class|ComboNode|GetComboName)))))) 0)
            (Variables|Default|SetStartPos (Utilities|Array|Get(acopy) (.StartPositions (Utilities|Struct|BreakWVConfig_ComboInfo (.Value (Utilities|Map|Find (Utilities|Struct|BreakWVConfig_ComboRow _returnvalue_2) (Class|ComboNode|GetComboName))))) (Class|ComboNode|GetComboIndex)))))
        (bind _returnvalue_3 (Utilities|LoadAssetBlocking (.ComboMontage (Utilities|Struct|BreakWVConfig_ComboInfo (.Value (Utilities|Map|Find (Utilities|Struct|BreakWVConfig_ComboRow _returnvalue_2) (Class|ComboNode|GetComboName)))))))
        (bind _asanim_montage (Utilities|Casting|CastToAnimMontage _returnvalue_3))
        (if (Utilities|Name|Equal(Name) (Variables|Default|GetSection) "None")
          (Animation|Montage|PlayMontage (Variables|/Script/Engine.Character|GetMesh (Variables|Default|GetActionCharacter)) _asanim_montage (Variables|Default|GetRate) (Variables|Default|GetStartPos))
          (else
            (Animation|Montage|PlayMontage (Variables|/Script/Engine.Character|GetMesh (Variables|Default|GetActionCharacter)) _asanim_montage (Variables|Default|GetRate) 0.0 (Variables|Default|GetSection))))))))

(fn Condition
  (bind _returnvalue (|CallParentFunction))
  (return _returnvalue))