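; Base equipment actor that turns hits reported by its hit collector into point damage, colored Niagara sparks and impact feedback.
; It binds a hit callback on BeginPlay, then looks up the owner's current combo action in the ComboAction config data table.
; That row can trigger a camera shake, played only for non-AI owners, and a timed, optionally delayed global slow-motion.
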(event Custom|HitCallback
  (params (HitResult :type Hit%20Result%20Structure%20%28by%20ref%29) (Causer :type Actor%20Object%20Reference) (CauserComp :type Actor%20Component%20Object%20Reference))
  (bind (_bblockinghit _binitialoverlap _time _distance _location _impactpoint _normal _impactnormal _physmat _hitactor) (Collision|BreakHitResult HitResult))
  (Game|Damage|ApplyPointDamage _hitactor 1.0 (* _impactnormal -1) HitResult (Pawn|GetController (Class|HitCollectorComp|GetOwnerCharacter (Variables|Default|Get_Comp_HitCollector))) Causer "/Script/Engine.DamageType")
  (bind _returnvalue (Niagara|SpawnSystematLocation "/Game/FX/NE_Spark_System.NE_Spark_System" _impactpoint (Math|Conversions|RotationFromXVector _impactnormal)))
  (Niagara|SetNiagaraVariable(LinearColor) _returnvalue "User.SparkColor" (Variables|Default|GetSparkColor))
  (bind _asaction_character (Utilities|Casting|CastToActionCharacter (Class|HitCollectorComp|GetOwnerCharacter (Variables|Default|Get_Comp_HitCollector))))
  (Utilities|IsValid (Class|ComboMachineComp|GetCurNode (Variables|/Script/SimpleARPG.ActionCharacter|Get_Comp_ComboMachine _asaction_character))
    (:Is%20Valid
      (bind _returnvalue_2 (Class|WVBlueprintFunctionLibrary|GetConfig "ComboAction"))
      (bind _returnvalue_3 (Utilities|GetDataTableRow _returnvalue_2 (Class|ActionCharacter|GetActionCharacterName _asaction_character))
        (:then
          (if (.ReturnValue (Utilities|Map|Find (Utilities|Struct|BreakWVConfig_ComboActionRow _returnvalue_3) (Class|ComboNode|GetComboActionName (Class|ComboMachineComp|GetCurNode (Variables|/Script/SimpleARPG.ActionCharacter|Get_Comp_ComboMachine _asaction_character)))))
            (if (.bShake (Utilities|Struct|BreakWVComboActionData (.Value (Utilities|Map|Find (Utilities|Struct|BreakWVConfig_ComboActionRow _returnvalue_3) (Class|ComboNode|GetComboActionName (Class|ComboMachineComp|GetCurNode (Variables|/Script/SimpleARPG.ActionCharacter|Get_Comp_ComboMachine _asaction_character)))))))
              (CallFunction|ShakeEvent))
            (if (> (.Dilation (Utilities|Struct|BreakWVComboActionSlomoData (.SlomoData (Utilities|Struct|BreakWVComboActionData (.Value (Utilities|Map|Find (Utilities|Struct|BreakWVConfig_ComboActionRow _returnvalue_3) (Class|ComboNode|GetComboActionName (Class|ComboMachineComp|GetCurNode (Variables|/Script/SimpleARPG.ActionCharacter|Get_Comp_ComboMachine _asaction_character))))))))) 0.0)
              (CallFunction|SlomoEvent (.Dilation (Utilities|Struct|BreakWVComboActionSlomoData (.SlomoData (Utilities|Struct|BreakWVComboActionData (.Value (Utilities|Map|Find (Utilities|Struct|BreakWVConfig_ComboActionRow _returnvalue_3) (Class|ComboNode|GetComboActionName (Class|ComboMachineComp|GetCurNode (Variables|/Script/SimpleARPG.ActionCharacter|Get_Comp_ComboMachine _asaction_character))))))))) (.Duration (Utilities|Struct|BreakWVComboActionSlomoData (.SlomoData (Utilities|Struct|BreakWVComboActionData (.Value (Utilities|Map|Find (Utilities|Struct|BreakWVConfig_ComboActionRow _returnvalue_3) (Class|ComboNode|GetComboActionName (Class|ComboMachineComp|GetCurNode (Variables|/Script/SimpleARPG.ActionCharacter|Get_Comp_ComboMachine _asaction_character))))))))) (.Delay (Utilities|Struct|BreakWVComboActionSlomoData (.SlomoData (Utilities|Struct|BreakWVComboActionData (.Value (Utilities|Map|Find (Utilities|Struct|BreakWVConfig_ComboActionRow _returnvalue_3) (Class|ComboNode|GetComboActionName (Class|ComboMachineComp|GetCurNode (Variables|/Script/SimpleARPG.ActionCharacter|Get_Comp_ComboMachine _asaction_character)))))))))))))))))

(event Custom|ShakeEvent
  (bind _returnvalue (Game|GetPlayerCameraManager 0))
  (if (Utilities|IsValidClass (Variables|Default|Get_Shake))
    (bind _asaction_character (Utilities|Casting|CastToActionCharacter (Class|HitCollectorComp|GetOwnerCharacter (Variables|Default|Get_Comp_HitCollector))))
    (Utilities|IsValid _asaction_character
      (:Is%20Valid
        (if (not (Variables|/Script/SimpleARPG.ActionCharacter|GetIsAI _asaction_character))
          (Utilities|IsValid _returnvalue
            (:Is%20Valid
              (Class|PlayerCameraManager|PlayCameraShake _returnvalue (Variables|Default|Get_Shake) 1.0 "CameraLocal" "0, 0, 0"))))))))

(event Custom|SlomoEvent
  (params (Dilation :type Float%20%28single-precision%29) (Duration :type Float%20%28single-precision%29) (Delay :type Float%20%28single-precision%29))
  (if (> Delay 0.0)
    (Utilities|FlowControl|Delay Delay))
  (Utilities|Time|SetGlobalTimeDilation Dilation)
  (Utilities|FlowControl|Delay Duration)
  (Utilities|Time|SetGlobalTimeDilation 1.0))

(event EventBeginPlay
  (EventDispatchers|AssignHitCallback (Variables|Default|Get_Comp_HitCollector) (delegate Custom|HitCallback)))

(event Collision|EventActorBeginOverlap
  (params (OtherActor :type Actor%20Object%20Reference)))

(event EventTick
  (params (DeltaSeconds :type Float%20%28single-precision%29)))

(fn ConstructionScript)