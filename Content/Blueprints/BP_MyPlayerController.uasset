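; Player controller that turns input actions into lock-target, sprint and dodge commands on the controlled BP_Player.
; A GetPlayer helper casts the controlled pawn to BP_Player and caches it for reuse.
; The HandlePostInput override calls the parent, then tries to start the player's combo machine and invalidates the input buffer when that succeeds.
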(event EventBeginPlay)

(event EventTick
  (params (DeltaSeconds :type Float%20%28single-precision%29)))

(event EventHandlePostInput
  ;[1 1 1] Handle Post Input
  (|CallParentFunction)
  (bind _bp_player (CallFunction|GetPlayer))
  (bind _returnvalue (Class|ComboMachineComp|Start (Class|ActionCharacter|GetComboMachineComp _bp_player)))
  (if _returnvalue
    (Class|InputBufferComp|Invalid (Variables|Default|Get_Comp_InputBuffer))))

(event Input|ActionEvents|InputActionX
  (params (Key :type Key%20Structure :default "None"))
  ;[1 1 1] Lock Target
  (:Pressed
    (CallFunction|GetPlayer)
    (Class|PlayerCharacter|LockTarget (Variables|Default|GetPlayerCharacter))))

(event Input|ActionEvents|InputActionA
  (params (Key :type Key%20Structure :default "None"))
  ;[1 1 1] Dodge
  (:Pressed
    (bind _bp_player (CallFunction|GetPlayer))
    (Class|ActionCharacter|Dodge _bp_player)))

(event Input|ActionEvents|InputActionR1
  (params (Key :type Key%20Structure :default "None"))
  ;[1 1 1] Sprint
  (:Pressed
    (CallFunction|GetPlayer)
    (Class|ActionCharacter|SetSprint (Variables|Default|GetPlayerCharacter) true))
  (:Released
    (CallFunction|GetPlayer)
    (Class|ActionCharacter|SetSprint (Variables|Default|GetPlayerCharacter) false)))

(fn ConstructionScript)

(fn GetPlayer
  (Utilities|IsValid (Variables|Default|GetPlayerCharacter)
    (:Is%20Valid
      _)
    (:Is%20Not%20Valid
      (bind _asbp_player (Utilities|Casting|CastToBP_Player (Pawn|GetControlledPawn)))
      (Variables|Default|SetPlayerCharacter _asbp_player)))
  (return (Variables|Default|GetPlayerCharacter)))